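; Playable ally character for turn-based grid battles, with camera controls, hover and selection highlights, and health.
; MoveRootComponent calls FindPath, a hand-written A*-style search around blocked cells and "Physical" actors, then steps through waypoints with MoveComponentTo.
; Click selection and Tab turn changes go through BattleState, and F damages the selected GenericEnemy.
; While active and idle, Tick flashes emitters over nearby cells based on Speed.
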(event Custom|OnClicked_Event
  (params (TouchedActor :type Actor%20Object%20Reference) (ButtonPressed :type Key%20Structure :default "None"))
  (bind _ascharacter (Utilities|Casting|CastToCharacter TouchedActor))
  (Default|ChangeSelectedCharacter (.AsBattle%20State (Utilities|Casting|CastToBattleState (Game|GetGameState))) _ascharacter))

(event Custom|OnBeginCursorOver_Event
  (params (TouchedActor :type Actor%20Object%20Reference))
  (Rendering|Material|SetOverlayMaterial (Variables|Character|GetMesh) "/Game/Stactic/OverlayMaterials/OverlayMaterial.OverlayMaterial" :!class /Script/Engine.MeshComponent))

(event Custom|OnEndCursorOver_Event
  (params (TouchedActor :type Actor%20Object%20Reference))
  (if (not (Variables|Default|GetSelectedActor))
    (Rendering|Material|SetOverlayMaterial (Variables|Character|GetMesh) 0 :!class /Script/Engine.MeshComponent)))

(event EventTick
  (params (DeltaSeconds :type Float%20%28single-precision%29))
  (bind _returnvalue (Game|GetGameMode))
  (bind _speed (Variables|Default|GetSpeed))
  (bind _asbp_top_down_game_mode (Utilities|Casting|CastToBP_TopDownGameMode _returnvalue))
  (bind _returnvalue_2 (* _speed 2))
  (bind _cellsize (Variables|/Game/Dynamic/Blueprints/BP_TopDownGameMode.BP_TopDownGameMode_C|GetCellSize _asbp_top_down_game_mode))
  (if (Variables|Default|GetIs%20it%20active?)
    (if (not (Variables|Default|GetIs%20it%20Moving?))
      (Utilities|FlowControl|Gate false) ; enters at Open
      (else
        (Utilities|FlowControl|Gate false) ; enters at Close
      ))))

(event EventBeginPlay
  (bind _returnvalue (Game|GetGameMode))
  (bind _returnvalue_2 (Game|GetPlayerController 0))
  (bind _self self)
  (bind _asbp_top_down_game_mode (Utilities|Casting|CastToBP_TopDownGameMode _returnvalue))
  (bind _rootcomponent (Variables|Transformation|GetRootComponent _self))
  (bind _returnvalue_3 (Transformation|GetWorldLocation _rootcomponent))
  (bind _cellsize (Variables|/Game/Dynamic/Blueprints/BP_TopDownGameMode.BP_TopDownGameMode_C|GetCellSize _asbp_top_down_game_mode))
  (bind (_x _y) (Math|Vector|BreakVector _returnvalue_3))
  (bind _returnvalue_4 (Math|Conversions|ToFloat(Integer) _cellsize))
  (Utilities|FlowControl|Sequence
    (:then_0)
    (:then_2
      (Variables|Default|SetX%20axis (Math|Float|Round (/ _x _returnvalue_4)))
      (Variables|Default|SetY%20axis (Math|Float|Round (/ _y _returnvalue_4))))
    (:then_3
      (Variables|/Script/Engine.PlayerController|SetbEnableMouseOverEvents _returnvalue_2 true)
      (Variables|/Script/Engine.PlayerController|SetbEnableClickEvents _returnvalue_2 true)
      (EventDispatchers|BindEventtoOnClicked (delegate Custom|OnClicked_Event))
      (EventDispatchers|BindEventtoOnBeginCursorOver (delegate Custom|OnBeginCursorOver_Event))
      (EventDispatchers|BindEventtoOnEndCursorOver (delegate Custom|OnEndCursorOver_Event)))))

(event Game|Damage|EventAnyDamage
  (params (Damage :type Float%20%28single-precision%29) (DamageType :type Damage%20Type%20Object%20Reference) (InstigatedBy :type Controller%20Object%20Reference) (DamageCauser :type Actor%20Object%20Reference))
  (bind _output_get (Variables|Default|SetHealth (- (Variables|Default|GetHealth) Damage)))
  (Development|PrintString (Utilities|String|ToString(Float) _output_get))
  (if (<= _output_get 0.0)
    (Utilities|FlowControl|Delay 0.2)
    (Actor|DestroyActor)))

(event EventMoveRootComponent
  (params (Location :type Vector :default "0, 0, 0"))
  (bind _locationstomove (Variables|Default|GetLocationsToMove))
  (bind _rootcomponent (Variables|Transformation|GetRootComponent))
  (bind _returnvalue (Transformation|GetWorldLocation _rootcomponent))
  (if (== (Game|Player|GetPlayerPawn 0) self)
    (if (Variables|Default|GetIs%20it%20Moving?)
      (Development|PrintString "Is moving")
      (else
        (Niagara|SpawnSystematLocation "/Game/Stactic/Cursor/FX_Cursor.FX_Cursor" Location)
        (CallFunction|FindPath Location)
        (if (Variables|Default|GetIs%20character%20already%20there?)
          _
          (else
            (Variables|Default|SetIs%20it%20Moving? true)
            (Transformation|SetWorldRotation (Variables|Character|GetMesh) (Math|Rotator|MakeRotator 0.0 0.0 (+ (.Yaw (Math|Rotator|BreakRotator (Math|Rotator|FindLookatRotation (Transformation|GetWorldLocation (Variables|Character|GetMesh self)) (Utilities|Array|Get(acopy) _locationstomove (Variables|Default|GetLocations%20to%20move%20array%20index))))) -9e+01)) false false :!label _label)
            (Components|MoveComponentTo _rootcomponent (Math|Vector|MakeVector (.X (Math|Vector|BreakVector (Utilities|Array|Get(acopy) _locationstomove (Variables|Default|GetLocations%20to%20move%20array%20index)))) (.Y (Math|Vector|BreakVector (Utilities|Array|Get(acopy) _locationstomove (Variables|Default|GetLocations%20to%20move%20array%20index)))) (.Z (Math|Vector|BreakVector _returnvalue))) "0, 0, 0" false false (/ (Math|Vector|Distance(Vector) (Utilities|Array|Get(acopy) _locationstomove (Variables|Default|GetLocations%20to%20move%20array%20index)) _returnvalue) (Variables|Default|GetWalking%20velocity)) true)
            (Math|Integer|IncrementInt (Variables|Default|GetLocations%20to%20move%20array%20index)
              (:%20%20
                (if (== (Utilities|Array|Length _locationstomove) (Variables|Default|GetLocations%20to%20move%20array%20index))
                  (Variables|Default|SetLocations%20to%20move%20array%20index 0)
                  (Utilities|Array|Clear (Variables|Default|GetLocationsToMove))
                  (Variables|Default|SetIs%20it%20Moving? false)
                  (else
                    (goto _label)))))))
        (Variables|Default|SetIs%20character%20already%20there? false)))
    (else
      (Development|PrintString "Inactive character"))))

(event EventPossessed
  (params (NewController :type Controller%20Object%20Reference)))

(event EventUnpossessed
  (params (OldController :type Controller%20Object%20Reference)))

(event EventSetActiveCharacter)

(event EventDefineXY
  (params (X%20axis :type Integer) (Y%20axis :type Integer))
  (Variables|Default|SetX%20axis X%20axis)
  (Variables|Default|SetY%20axis Y%20axis))

(event EventChangeSelectedMaterial
  (params (On%20or%20Off? :type Boolean))
  (bind _mesh (Variables|Character|GetMesh))
  (bind _output_get (Variables|Default|SetSelectedActor On%20or%20Off?))
  (if _output_get
    (Rendering|Material|SetOverlayMaterial _mesh "/Game/Stactic/OverlayMaterials/SelectedMaterial.SelectedMaterial" :!class /Script/Engine.MeshComponent)
    (else
      (Rendering|Material|SetOverlayMaterial _mesh 0 :!class /Script/Engine.MeshComponent))))

(event Input|MouseEvents|MiddleMouseButton
  (params (Key :type Key%20Structure)))

(event Input|KeyboardEvents|Tab
  (params (Key :type Key%20Structure))
  (:Pressed
    (Development|PrintString "Tab Pressed")
    (if (== (Game|Player|GetPlayerPawn 0) self)
      (Default|ChangeCharacterTurn (.AsBattle%20State (Utilities|Casting|CastToBattleState (Game|GetGameState)))))))

(event Input|MouseEvents|MouseWheelDown
  (params (Key :type Key%20Structure))
  (bind _springarm (Variables|Camera|GetSpringArm))
  (:Pressed
    (if (== (Game|Player|GetPlayerPawn 0) self)
      (if (not (> (Variables|/Script/Engine.SpringArmComponent|GetTargetArmLength _springarm) 2999.0))
        (Variables|/Script/Engine.SpringArmComponent|SetTargetArmLength _springarm (+ (Variables|/Script/Engine.SpringArmComponent|GetTargetArmLength _springarm) 5e+01))))))

(event Input|MouseEvents|MouseWheelUp
  (params (Key :type Key%20Structure))
  (bind _springarm (Variables|Camera|GetSpringArm))
  (:Pressed
    (if (== (Game|Player|GetPlayerPawn 0) self)
      (if (not (< (Variables|/Script/Engine.SpringArmComponent|GetTargetArmLength _springarm) 201.0))
        (Variables|/Script/Engine.SpringArmComponent|SetTargetArmLength _springarm (+ (Variables|/Script/Engine.SpringArmComponent|GetTargetArmLength _springarm) -5e+01))))))

(event Input|KeyboardEvents|NumPadZero
  (params (Key :type Key%20Structure))
  (bind _camera (Variables|Camera|GetCamera))
  (bind _camera_2 (Variables|Camera|GetCamera))
  (bind _camera_3 (Variables|Camera|GetCamera))
  (:Pressed
    (if (== (Game|Player|GetPlayerPawn 0) self)
      (if (not (Variables|Default|GetIsCameraMoving?))
        (Variables|Default|SetIsCameraMoving? true)
        (switch int (Variables|Default|GetCamera%20selection)
          (:0
            (Components|MoveComponentTo _camera_3 (+ (Variables|/Script/Engine.SceneComponent|GetRelativeLocation _camera_3) "-300.000000,850.000000,-400.000000") (Variables|/Script/Engine.SceneComponent|GetRelativeRotation (Variables|Default|GetCamera0)) true true (Variables|Default|GetCamera%20speed) false)
            (Math|Integer|IncrementInt (Variables|Default|GetCamera%20selection)
              (:%20%20
                _)))
          (:1
            (Components|MoveComponentTo _camera_2 (+ (Variables|/Script/Engine.SceneComponent|GetRelativeLocation _camera_2) "300.000000,850.000000,400.000000") (Variables|/Script/Engine.SceneComponent|GetRelativeRotation (Variables|Default|GetCamera1)) true true (Variables|Default|GetCamera%20speed) false)
            (Math|Integer|IncrementInt (Variables|Default|GetCamera%20selection)
              (:%20%20
                _)))
          (:2
            (Components|MoveComponentTo _camera (+ (Variables|/Script/Engine.SceneComponent|GetRelativeLocation _camera) "0,-1700.000000,0.000000") (Variables|/Script/Engine.SceneComponent|GetRelativeRotation (Variables|Default|GetCamera2)) true true (Variables|Default|GetCamera%20speed) false)
            (Variables|Default|SetCamera%20selection 0)))
        (Variables|Default|SetIsCameraMoving? false)))))

(event Input|KeyboardEvents|NumPadOne
  (params (Key :type Key%20Structure))
  (:Pressed
    (if (== (Game|Player|GetPlayerPawn 0) self)
      (Transformation|SetRelativeTransform (Variables|Camera|GetCamera) (Variables|Default|GetCamera%20inital%20transform) false false)
      (Variables|Default|SetCamera%20selection 1))))

(event Input|KeyboardEvents|F
  (params (Key :type Key%20Structure))
  (:Pressed
    (bind _asgeneric_enemy (Utilities|Casting|CastToGenericEnemy (Variables|/Game/Dynamic/BattleState.BattleState_C|GetSelectedCharacter (.AsBattle%20State (Utilities|Casting|CastToBattleState (Game|GetGameState))))))
    (Game|Damage|ApplyDamage _asgeneric_enemy 3.0 0 0)))

(fn ConstructionScript)

(fn FindPath
  (params (Target%20location :type Vector))
  (bind _returnvalue (Game|GetPlayerCharacter 0))
  (bind (_x _y _z) (Math|Vector|BreakVector Target%20location))
  (bind _nexttoprevious (LocalVariables|GetNextToPrevious))
  (bind _nexttoprevious_2 (LocalVariables|GetNextToPrevious))
  (bind _returnvalue_2 (Math|Float|Round _y))
  (bind _returnvalue_3 (Math|Float|Round _x))
  (bind _returnvalue_4 (Transformation|GetActorLocation _returnvalue))
  (bind _returnvalue_5 (Math|Conversions|ToFloat(Integer) _returnvalue_2))
  (bind _returnvalue_6 (Math|Conversions|ToFloat(Integer) _returnvalue_3))
  (LocalVariables|SetNextNeighboor _returnvalue_4)
  (Utilities|Array|Clear (Variables|Default|GetLocationsToMove))
  (bind _outactors (Actor|GetAllActorswithTag "Physical"))
  (bind _array_element (Utilities|Array|ForEachLoopwithBreak _outactors :!label _label)
    (:LoopBody
      (if (Utilities|Operators|EqualEqual Target%20location (Math|Vector|MakeVector (.x (Transformation|GetActorLocation _array_element)) (.y (Transformation|GetActorLocation _array_element)) 0.0) 0.01)
        (Variables|Default|SetIs%20character%20already%20there? true)
        (goto _label Break)
        (else
          (Utilities|Array|Add (LocalVariables|GetOtherPhysicalActorLocations) (Math|Vector|MakeVector (.x (Transformation|GetActorLocation _array_element)) (.y (Transformation|GetActorLocation _array_element)) 0.0)))))
    (:Completed
      (if (Variables|Default|GetIs%20character%20already%20there?)
        (Development|PrintString "There is a character there" true true "(R=0.265625,G=0.099744,B=0.078857,A=1.000000)")
        (else
          (bind _returnvalue_7 (Actor|GetActorOfClass "/Game/Dynamic/GridIndexMap1.GridIndexMap1_C"))
          (Variables|Default|SetBlocked%20Locations (Variables|/Game/Dynamic/GridIndexMap1.GridIndexMap1_C|GetBlockedLocations _returnvalue_7))
          (LocalVariables|SetRoot%20component%20Z%20value (.Z (Math|Vector|BreakVector _returnvalue_4)))
          (LocalVariables|SetCell%20size (Variables|/Game/Dynamic/Blueprints/BP_TopDownGameMode.BP_TopDownGameMode_C|GetCellSize (.AsBP%20Top%20Down%20Game%20Mode (Utilities|Casting|CastToBP_TopDownGameMode (Game|GetGameMode)))))
          (LocalVariables|SetX%20neighboor%20axis (Variables|Default|GetX%20axis))
          (LocalVariables|SetY%20neighboor%20axis (Variables|Default|GetY%20axis))
          (for _index (range 0 2) :!label _label_2
            (for _index_2 (range 0 2)
              (if (not (or (Utilities|Array|ContainsItem (Variables|Default|GetBlocked%20Locations) (Math|Vector|MakeVector (Math|Conversions|ToFloat(Integer) (* (+ (+ (LocalVariables|GetX%20neighboor%20axis) -1) _index) (LocalVariables|GetCell%20size))) (Math|Conversions|ToFloat(Integer) (* (+ (+ (LocalVariables|GetY%20neighboor%20axis) -1) _index_2) (LocalVariables|GetCell%20size))) 0.0)) (Utilities|Array|ContainsItem (LocalVariables|GetOtherPhysicalActorLocations) (Math|Vector|MakeVector (Math|Conversions|ToFloat(Integer) (* (+ (+ (LocalVariables|GetX%20neighboor%20axis) -1) _index) (LocalVariables|GetCell%20size))) (Math|Conversions|ToFloat(Integer) (* (+ (+ (LocalVariables|GetY%20neighboor%20axis) -1) _index_2) (LocalVariables|GetCell%20size))) 0.0))))
                (Utilities|Map|Add (LocalVariables|GetOpenNodes) (Math|Vector|MakeVector (Math|Conversions|ToFloat(Integer) (* (+ (+ (LocalVariables|GetX%20neighboor%20axis) -1) _index) (LocalVariables|GetCell%20size))) (Math|Conversions|ToFloat(Integer) (* (+ (+ (LocalVariables|GetY%20neighboor%20axis) -1) _index_2) (LocalVariables|GetCell%20size))) (LocalVariables|GetRoot%20component%20Z%20value)) (Math|Vector|MakeVector (Math|Conversions|ToFloat(Integer) (+ (Math|Integer|SelectInt (+ 0 14) (+ 0 10) (and (or (== (+ (+ (LocalVariables|GetX%20neighboor%20axis) -1) _index) (+ (LocalVariables|GetX%20neighboor%20axis) 1)) (== (+ (+ (LocalVariables|GetX%20neighboor%20axis) -1) _index) (- (LocalVariables|GetX%20neighboor%20axis) 1))) (or (== (+ (+ (LocalVariables|GetY%20neighboor%20axis) -1) _index_2) (+ (LocalVariables|GetY%20neighboor%20axis) 1)) (== (+ (+ (LocalVariables|GetY%20neighboor%20axis) -1) _index_2) (- (LocalVariables|GetY%20neighboor%20axis) 1))))) (* (/ (Math|Float|Round (Math|Vector|Distance2D(Vector) (Math|Vector|MakeVector (Math|Conversions|ToFloat(Integer) (* (+ (+ (LocalVariables|GetX%20neighboor%20axis) -1) _index) (LocalVariables|GetCell%20size))) (Math|Conversions|ToFloat(Integer) (* (+ (+ (LocalVariables|GetY%20neighboor%20axis) -1) _index_2) (LocalVariables|GetCell%20size))) (LocalVariables|GetRoot%20component%20Z%20value)) (Math|Vector|MakeVector _returnvalue_6 _returnvalue_5 (+ _z (LocalVariables|GetRoot%20component%20Z%20value))))) (LocalVariables|GetCell%20size)) 10))) (Math|Conversions|ToFloat(Integer) (* (/ (Math|Float|Round (Math|Vector|Distance2D(Vector) (Math|Vector|MakeVector (Math|Conversions|ToFloat(Integer) (* (+ (+ (LocalVariables|GetX%20neighboor%20axis) -1) _index) (LocalVariables|GetCell%20size))) (Math|Conversions|ToFloat(Integer) (* (+ (+ (LocalVariables|GetY%20neighboor%20axis) -1) _index_2) (LocalVariables|GetCell%20size))) (LocalVariables|GetRoot%20component%20Z%20value)) (Math|Vector|MakeVector _returnvalue_6 _returnvalue_5 (+ _z (LocalVariables|GetRoot%20component%20Z%20value))))) (LocalVariables|GetCell%20size)) 10)) (Math|Conversions|ToFloat(Integer) (Math|Integer|SelectInt (+ 0 14) (+ 0 10) (and (or (== (+ (+ (LocalVariables|GetX%20neighboor%20axis) -1) _index) (+ (LocalVariables|GetX%20neighboor%20axis) 1)) (== (+ (+ (LocalVariables|GetX%20neighboor%20axis) -1) _index) (- (LocalVariables|GetX%20neighboor%20axis) 1))) (or (== (+ (+ (LocalVariables|GetY%20neighboor%20axis) -1) _index_2) (+ (LocalVariables|GetY%20neighboor%20axis) 1)) (== (+ (+ (LocalVariables|GetY%20neighboor%20axis) -1) _index_2) (- (LocalVariables|GetY%20neighboor%20axis) 1)))))))))))
          (Utilities|Array|Add (LocalVariables|GetAlreadyUsedCoordinates) (LocalVariables|GetNextNeighboor))
          (bind _values (Utilities|Map|Values (LocalVariables|GetOpenNodes)))
          (for _array_element_2 _values
            (if (< (Math|Float|Round (.X (Math|Vector|BreakVector _array_element_2))) (Math|Float|Round (.X (Math|Vector|BreakVector (LocalVariables|GetLowestValue)))))
              (if (== (Math|Float|Round (.X (Math|Vector|BreakVector (LocalVariables|GetLowestValue)))) (Math|Float|Round (.X (Math|Vector|BreakVector _array_element_2))))
                (if (< (Math|Float|Round (.Y (Math|Vector|BreakVector _array_element_2))) (Math|Float|Round (.Y (Math|Vector|BreakVector (LocalVariables|GetLowestValue)))))
                  (LocalVariables|SetLowestValue _array_element_2 :!label _label_3))
                (else
                  (goto _label_3)))))
          (LocalVariables|SetMoveCost (Math|Float|Round (.Z (Math|Vector|BreakVector (LocalVariables|GetLowestValue)))))
          (bind _keys (Utilities|Map|Keys (LocalVariables|GetOpenNodes)))
          (bind _array_element_3 (Utilities|Array|ForEachLoopwithBreak _keys :!label _label_4)
            (:LoopBody
              (if (Utilities|Operators|EqualEqual (.Value (Utilities|Map|Find (LocalVariables|GetOpenNodes) _array_element_3)) (LocalVariables|GetLowestValue) 0.01)
                (if (not (Math|Boolean|ORBoolean (Utilities|Array|ContainsItem (LocalVariables|GetAlreadyUsedCoordinates) _array_element_3) (Utilities|Array|ContainsItem (Variables|Default|GetBlocked%20Locations) _array_element_3) (Utilities|Array|ContainsItem (LocalVariables|GetOtherPhysicalActorLocations) _array_element_3)))
                  (bind _output_get (LocalVariables|SetPreviousNeighboor (LocalVariables|GetNextNeighboor)))
                  (bind _output_get_2 (LocalVariables|SetNextNeighboor _array_element_3))
                  (goto _label_4 Break)
                  (else
                    (Development|PrintString "Blocked")))))
            (:Completed
              (LocalVariables|SetX%20neighboor%20axis (Math|Float|Round (/ (.X (Math|Vector|BreakVector (LocalVariables|GetNextNeighboor))) (Math|Conversions|ToFloat(Integer) (LocalVariables|GetCell%20size)))))
              (LocalVariables|SetY%20neighboor%20axis (Math|Float|Round (/ (.Y (Math|Vector|BreakVector (LocalVariables|GetNextNeighboor))) (Math|Conversions|ToFloat(Integer) (LocalVariables|GetCell%20size)))))
              (for _array_element_4 (LocalVariables|GetAlreadyUsedCoordinates)
                (if (< (Math|Vector|Distance2D(Vector) _array_element_4 (LocalVariables|GetNextNeighboor)) (Math|Vector|Distance2D(Vector) (LocalVariables|GetClosest%20Node%20path%20purposes) (LocalVariables|GetNextNeighboor)))
                  (LocalVariables|SetClosest%20Node%20path%20purposes _array_element_4)))
              (if (== (Utilities|Map|Length _nexttoprevious) 0)
                (LocalVariables|SetFirstCalculatedCoordenate (LocalVariables|GetNextNeighboor)))
              (Utilities|Map|Add _nexttoprevious (LocalVariables|GetNextNeighboor) (LocalVariables|GetClosest%20Node%20path%20purposes))
              (if (Utilities|Operators|EqualEqual (LocalVariables|GetNextNeighboor) (Math|Vector|MakeVector _returnvalue_6 _returnvalue_5 (+ _z (LocalVariables|GetRoot%20component%20Z%20value))) 0.01)
                (LocalVariables|SetReverseCount (Math|Vector|MakeVector _returnvalue_6 _returnvalue_5 (+ _z (LocalVariables|GetRoot%20component%20Z%20value))))
                (bind _keys_2 (Utilities|Map|Keys _nexttoprevious_2))
                (for _array_element_5 _keys_2
                  (bind _output_get_3 (LocalVariables|SetReverseCount (.Value (Utilities|Map|Find _nexttoprevious_2 (LocalVariables|GetReverseCount)))))
                  (Utilities|Array|Add (LocalVariables|GetLocationsToMoveReversed) _output_get_3))
                (bind _arrayelement (Utilities|Array|ReverseforEachLoop (LocalVariables|GetLocationsToMoveReversed))
                  (:LoopBody
                    (Utilities|Array|Add (Variables|Default|GetLocationsToMove) _arrayelement))
                  (:Completed
                    (Utilities|Array|Add (Variables|Default|GetLocationsToMove) (Math|Vector|MakeVector _returnvalue_6 _returnvalue_5 (+ _z (LocalVariables|GetRoot%20component%20Z%20value))))))
                (else
                  (goto _label_2))))))))))